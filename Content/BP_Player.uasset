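; Player character Blueprint that turns input into movement, camera look, jumping, crouching and two kinds of shooting.
; Sprint is a held flag that lets forward/backward input through at full scale, which is otherwise halved; strafing follows control rotation.
; Shoot runs a debug-drawn multi line trace from BulletSpawn without using the hits, while ShootProjectile spawns BP_Ammo at the same transform.
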(event `InputAction|Sprint`
  (params (Key :type "Key Structure"))
  ;[0.0565 0.03535 0.15 0.5] Movment
  (:`Pressed`
    (set `self.Sprint` true))
  (:`Released`
    (set `self.Sprint` false)))

(event `InputAction|Jump`
  (params (Key :type "Key Structure"))
  ;[0.0565 0.03535 0.15 0.5] Movment
  (:`Pressed`
    (`self.Jump`)))

(event `InputAction|Shoot`
  (params (Key :type "Key Structure"))
  (bind (_returnvalue_location _returnvalue_rotation) (`KismetMathLibrary.BreakTransform` (`SceneComponent.K2_GetComponentToWorld` (`self.BulletSpawn`))))
  ;[0.15 0.04388 0.04251 0.5] Attack
  (:`Pressed`
    (`KismetSystemLibrary.LineTraceMulti` :`Start` _returnvalue_location :`End` (+ _returnvalue_location (* (`KismetMathLibrary.GetForwardVector` _returnvalue_rotation) (`self.Range`))) :`TraceChannel` "TraceTypeQuery1" :`bTraceComplex` true :`DrawDebugType` "ForDuration" :`DrawTime` 0.5)))

(event `InputAction|Crouch`
  (params (Key :type "Key Structure"))
  ;[0.0565 0.03535 0.15 0.5] Movment
  (:`Pressed`
    (`self.Crouch`))
  (:`Released`
    (`self.UnCrouch`)))

(event `InputAction|ShootProjectile`
  (params (Key :type "Key Structure"))
  (bind (_returnvalue_location _returnvalue_rotation) (`KismetMathLibrary.BreakTransform` (`SceneComponent.K2_GetComponentToWorld` (`self.BulletSpawn`))))
  ;[0.15 0.04388 0.04251 0.5] Attack
  (:`Pressed`
    (`|SpawnActorFromClass` "/Game/BP_Ammo.BP_Ammo_C" (`KismetMathLibrary.MakeTransform` _returnvalue_location _returnvalue_rotation) "Undefined" "MultiplyWithRoot" null null)))

(event `InputAxis|Left/Right`
  (params (AxisValue :type "Float (single-precision)"))
  (bind (_returnvalue_roll _returnvalue_pitch _returnvalue_yaw) (`KismetMathLibrary.BreakRotator` (`self.GetControlRotation`)))
  ;[0.0565 0.03535 0.15 0.5] Movment
  (`self.AddMovementInput` (`KismetMathLibrary.GetRightVector` (`KismetMathLibrary.MakeRotator` _returnvalue_roll 0.0 _returnvalue_yaw)) AxisValue))

(event `InputAxis|Forward/Backward`
  (params (AxisValue :type "Float (single-precision)"))
  (bind _returnvalue (`self.GetActorForwardVector`))
  ;[0.0565 0.03535 0.15 0.5] Movment
  (if (`self.Sprint`)
    (`self.AddMovementInput` _returnvalue AxisValue)
    (else
      (`self.AddMovementInput` _returnvalue (/ AxisValue 2.0)))))

(event `InputAxis|Camera_Top/Down`
  (params (AxisValue :type "Float (single-precision)"))
  ;[0.04032 0.04305 0.15 0.5] Camera Movment
  (`self.AddControllerPitchInput` AxisValue))

(event `InputAxis|Camera_Left/RIght`
  (params (AxisValue :type "Float (single-precision)"))
  ;[0.04032 0.04305 0.15 0.5] Camera Movment
  (`self.AddControllerYawInput` AxisValue))

(fn `UserConstructionScript`)